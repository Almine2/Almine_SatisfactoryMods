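; Explosive variant of the Jace Snutt pillow that pairs itself with a tiny Nobelisk cluster actor.
; On Hit it spawns the cluster at the supplied component's location with no lifespan limit and projectile movement tick disabled.
; Tick moves the stored cluster when the pillow's location differs from the cached one.
; The cluster is destroyed with the pillow and before saves, then respawned at the cached location after saving.
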(event `self.ReceiveBeginPlay`)

(event `self.ReceiveTick`
  (params (DeltaSeconds :type "Float (single-precision)"))
  (bind _returnvalue (`self.K2_GetActorLocation`))
  (if (!= _returnvalue (`self.Trans`) :`ErrorTolerance` 0.1)
    (`self.K2_SetActorRelativeLocation` (`self.cluster`) _returnvalue false false)
    (set `self.Trans` _returnvalue)))

(event `self.ReceiveHit`
  (params (MyComp :type "PrimitiveComponent Object Reference") (Other :type "Actor Object Reference") (OtherComp :type "PrimitiveComponent Object Reference") (bSelfMoved :type Boolean) (HitLocation :type "Vector Structure") (HitNormal :type "Vector Structure") (NormalImpulse :type "Vector Structure") (Hit :type "HitResult Structure (by ref)"))
  (bind _returnvalue (`SceneComponent.K2_GetComponentLocation` MyComp))
  (set `self.Trans` _returnvalue)
  (bind _returnvalue_2 (`|SpawnActorFromClass` "/Game/FactoryGame/Equipment/NobeliskDetonator/Ammo/BP_NobeliskCluster.BP_NobeliskCluster_C" (`KismetMathLibrary.MakeTransform` _returnvalue (struct) (0.05 0.05 0.05)) "AlwaysSpawn" "MultiplyWithRoot" null null))
  (`self.SetActorHiddenInGame` _returnvalue_2 false)
  (`self.SetLifeSpan` _returnvalue_2 -1.0)
  (`ActorComponent.SetComponentTickEnabled` (`FGProjectile.mProjectileMovement` _returnvalue_2) false)
  (set `self.cluster` _returnvalue_2))

(event `self.ReceiveDestroyed`
  (bind _cluster (`self.cluster`))
  (if (`KismetSystemLibrary.IsValid` _cluster)
    (`self.K2_DestroyActor` _cluster)))

(event `FGSaveInterface.PreSaveGame`
  (params (saveVersion :type Integer) (gameVersion :type Integer))
  (bind _cluster (`self.cluster`))
  (if (`KismetSystemLibrary.IsValid` _cluster)
    (`self.K2_DestroyActor` _cluster)))

(event `FGSaveInterface.PostSaveGame`
  (params (saveVersion :type Integer) (gameVersion :type Integer))
  (bind _returnvalue (`|SpawnActorFromClass` "/Game/FactoryGame/Equipment/NobeliskDetonator/Ammo/BP_NobeliskCluster.BP_NobeliskCluster_C" (`KismetMathLibrary.MakeTransform` (`self.Trans`) (struct) (0.05 0.05 0.05)) "AlwaysSpawn" "MultiplyWithRoot" null null))
  (`self.SetActorHiddenInGame` _returnvalue false)
  (`self.SetLifeSpan` _returnvalue -1.0)
  (`ActorComponent.SetComponentTickEnabled` (`FGProjectile.mProjectileMovement` _returnvalue) false)
  (set `self.cluster` _returnvalue))

(fn `UserConstructionScript`
  (`parent.UserConstructionScript`))